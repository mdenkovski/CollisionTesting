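; BP_MaterialListener is an actor that keeps its static mesh materials in sync with the current quality level.
; On BeginPlay it replaces each mesh material with a dynamic instance, stores them, and binds to the ScreenPercentageManager's quality change event if that manager is valid.
; When the level changes, it saves the value and pushes it to every instance as the "Quality" scalar parameter, with debug prints along the way.
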(event Custom|QualityLevelChanged
  (params (Quality :type Float%20%28single-precision%29))
  (Variables|Default|SetQuality Quality)
  (Development|PrintString "quality level updated")
  (for _array_element (Variables|Default|GetDynamicMaterials)
    (Rendering|Material|SetScalarParameterValue _array_element "Quality" (Variables|Default|GetQuality) :!class /Script/Engine.MaterialInstanceDynamic)))

(event EventBeginPlay
  (bind _staticmesh (Variables|Default|GetStaticMesh))
  (bind _screenpercentagemanager (Variables|Default|GetScreenPercentageManager))
  (for (_array_element _array_index) (Rendering|Material|GetMaterials _staticmesh)
    (bind _returnvalue (Rendering|Material|CreateDynamicMaterialInstance _staticmesh _array_index _array_element "None" :!class /Script/Engine.PrimitiveComponent))
    (bind _returnvalue_2 (Utilities|Array|Add (Variables|Default|GetDynamicMaterials) _returnvalue))
    (Development|PrintString (Utilities|String|Append "created material instance for material element: " (Utilities|String|ToString(Integer) _returnvalue_2))))
  (Utilities|IsValid _screenpercentagemanager
    (:Is%20Valid
      (EventDispatchers|BindEventtoQualityLevelChanged _screenpercentagemanager (delegate Custom|QualityLevelChanged)))))

(event Collision|EventActorBeginOverlap
  (params (OtherActor :type Actor%20Object%20Reference)))

(event EventTick
  (params (DeltaSeconds :type Float%20%28single-precision%29)))

(fn ConstructionScript)